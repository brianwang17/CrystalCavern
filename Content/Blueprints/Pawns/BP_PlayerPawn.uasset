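; BP_PlayerPawn is a player pawn that moves by applying physics torque to its Mesh.
; The two movement axis inputs torque the Mesh around Y for forwards/backwards and X for right/left, scaled by AccelerationMultiplier.
; Torque is applied as an acceleration change, so the response ignores mass.
; On BeginPlay, the player camera manager starts a short fade from solid white.
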(event `InputAxis|Move Forwards/Backwards`
  (params (AxisValue :type "Float (single-precision)"))
  (`PrimitiveComponent.AddTorqueInRadians` (`self.Mesh`) (`KismetMathLibrary.MakeVector` 0.0 (* AxisValue (`self.Acceleration Multiplier`))) "None" true))

(event `InputAxis|Move Right/Left`
  (params (AxisValue :type "Float (single-precision)"))
  (`PrimitiveComponent.AddTorqueInRadians` (`self.Mesh`) (`KismetMathLibrary.MakeVector` (* AxisValue (`self.Acceleration Multiplier`))) "None" true))

(event `self.ReceiveBeginPlay`
  (`PlayerCameraManager.StartCameraFade` (`GameplayStatics.GetPlayerCameraManager` 0) 1.0 0.0 0.5 (struct :`R` 1.0 :`G` 1.0 :`B` 1.0 :`A` 1.0) false false))

(fn `UserConstructionScript`)